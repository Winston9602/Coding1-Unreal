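; Elevator platform actor that moves between Top and Bottom points when the third-person character enters its trigger volumes.
; Call triggers move it at once, while Send triggers wait briefly first, then share the same logic.
; IsMoving and IsBottom flags gate each trip, printing its direction.
; One timeline lerps the platform's world location, playing forward to rise and reversing to descend.
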(event `self.(col.) callTop.OnComponentBeginOverlap`
  (params (OverlappedComponent :type "PrimitiveComponent Object Reference") (OtherActor :type "Actor Object Reference") (OtherComp :type "PrimitiveComponent Object Reference") (OtherBodyIndex :type Integer) (bFromSweep :type Boolean) (SweepResult :type "HitResult Structure (by ref)"))
  ;[1 1 1] Brings the platform to the top if a player approaches the top of the elevator, or if they step onto the platform when it is at the bottom
  (cast `/Game/ThirdPersonBP/Blueprints/ThirdPersonCharacter` OtherActor)
  ;[1 1 1] If platform is not moving and IS at the bottom, continue and invert both of those variable checks
  (if (`self.isMoving`) :!label _label
    _
    (elif (`self.isBottom`)
      (set `self.isMoving` true)
      (set `self.isBottom` false)
      (`KismetSystemLibrary.PrintString` "Going up!")
      ;[1 1 1] LERP timeline to move the platform to/from either the Top or Bottom locations, depending on which location the player triggered
      (bind (_direction _newtrack_1) (`Timeline|Timeline_0` :!via `PlayFromStart` :!label _label_2)
        (:`Update`
          (bind _returnvalue_location (`KismetMathLibrary.BreakTransform` (`KismetMathLibrary.TLerp` (`SceneComponent.K2_GetComponentToWorld` (`self.Bottom`)) (`SceneComponent.K2_GetComponentToWorld` (`self.Top`)) _newtrack_1)))
          (`SceneComponent.K2_SetWorldLocation` (`self.Platform`) _returnvalue_location false false))
        (:`Finished`
          (set `self.isMoving` false))))))

(event `self.(col.) sendB-to-T.OnComponentBeginOverlap`
  (params (OverlappedComponent :type "PrimitiveComponent Object Reference") (OtherActor :type "Actor Object Reference") (OtherComp :type "PrimitiveComponent Object Reference") (OtherBodyIndex :type Integer) (bFromSweep :type Boolean) (SweepResult :type "HitResult Structure (by ref)"))
  ;[1 1 1] Brings the platform to the top if a player approaches the top of the elevator, or if they step onto the platform when it is at the bottom
  (cast `/Game/ThirdPersonBP/Blueprints/ThirdPersonCharacter` OtherActor)
  (`KismetSystemLibrary.Delay` 1.0)
  (goto _label))

(event `self.(col.) callBottom.OnComponentBeginOverlap`
  (params (OverlappedComponent :type "PrimitiveComponent Object Reference") (OtherActor :type "Actor Object Reference") (OtherComp :type "PrimitiveComponent Object Reference") (OtherBodyIndex :type Integer) (bFromSweep :type Boolean) (SweepResult :type "HitResult Structure (by ref)"))
  ;[1 1 1] Same as above, but vice versa for sending the platform to the bottom
  (cast `/Game/ThirdPersonBP/Blueprints/ThirdPersonCharacter` OtherActor)
  ;[1 1 1] If platform is not moving and is NOT at the bottom, continue and invert both of those variable checks
  (if (`self.isMoving`) :!label _label_3
    _
    (elif (not (`self.isBottom`))
      (set `self.isMoving` true)
      (set `self.isBottom` true)
      (`KismetSystemLibrary.PrintString` "Going down!")
      (goto _label_2 :!via `Reverse`))))

(event `self.(col.) sendT-to-B.OnComponentBeginOverlap`
  (params (OverlappedComponent :type "PrimitiveComponent Object Reference") (OtherActor :type "Actor Object Reference") (OtherComp :type "PrimitiveComponent Object Reference") (OtherBodyIndex :type Integer) (bFromSweep :type Boolean) (SweepResult :type "HitResult Structure (by ref)"))
  ;[1 1 1] Same as above, but vice versa for sending the platform to the bottom
  (cast `/Game/ThirdPersonBP/Blueprints/ThirdPersonCharacter` OtherActor)
  (`KismetSystemLibrary.Delay` 0.5)
  (goto _label_3))

(fn `UserConstructionScript`)