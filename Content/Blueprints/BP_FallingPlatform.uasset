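; Falling platform that drops after a ThirdPersonCharacter steps on its trigger box, then returns to its start position.
; A ready flag blocks retriggering while it runs a delayed sequence: activate, fall with physics simulation, then reset.
; Reset disables physics and uses a timeline to lerp the fallen transform back to the transform saved at BeginPlay.
; Each state swaps the platform material and prints a debug message.
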(event `self.ReceiveBeginPlay`
  (set `self.Starting Transform` (`SceneComponent.K2_GetComponentToWorld` (`self.Platform`)))
  (set `self.isReady` true)
  (`PrimitiveComponent.SetMaterial` (`self.Platform`) 0 "/Game/Materials/MI_PlatformReady.MI_PlatformReady"))

(event `self.Box Trigger.OnComponentBeginOverlap`
  (params (OverlappedComponent :type "PrimitiveComponent Object Reference") (OtherActor :type "Actor Object Reference") (OtherComp :type "PrimitiveComponent Object Reference") (OtherBodyIndex :type Integer) (bFromSweep :type Boolean) (SweepResult :type "HitResult Structure (by ref)"))
  (`KismetSystemLibrary.PrintString` "Something is standing on the platform")
  (if (`self.isReady`)
    (cast `/Game/ThirdPersonBP/Blueprints/ThirdPersonCharacter` OtherActor)
    (`self.Activate`)))

(event `Activate`
  (`PrimitiveComponent.SetMaterial` (`self.Platform`) 0 "/Game/Materials/MI_PlatformActivated.MI_PlatformActivated")
  (set `self.isReady` false)
  (`KismetSystemLibrary.PrintString` "Starting Countdown")
  (`KismetSystemLibrary.Delay` (`self.Fall Delay Duration`))
  (`self.Falling`))

(event `Falling`
  (`PrimitiveComponent.SetMaterial` (`self.Platform`) 0 "/Game/Materials/MI_PlatformFalling.MI_PlatformFalling")
  (`KismetSystemLibrary.PrintString` "Falling!")
  (`PrimitiveComponent.SetSimulatePhysics` (`self.Platform`) true)
  (`KismetSystemLibrary.Delay` (`self.Fall Duration`))
  (`self.Reset`))

(event `Reset`
  (`PrimitiveComponent.SetMaterial` (`self.Platform`) 0 "/Game/Materials/MI_PlatformResetting.MI_PlatformResetting")
  (`KismetSystemLibrary.PrintString` "Resetting the platform")
  (`PrimitiveComponent.SetSimulatePhysics` (`self.Platform`) false)
  (set `self.FallenTransform` (`SceneComponent.K2_GetComponentToWorld` (`self.Platform`)))
  (bind (_direction _newtrack_0) (`Timeline|GoBackToStartTransform` :!via `PlayFromStart`)
    (:`Update`
      (`SceneComponent.K2_SetWorldTransform` (`self.Platform`) (`KismetMathLibrary.TLerp` (`self.FallenTransform`) (`self.Starting Transform`) _newtrack_0) false false))
    (:`Finished`
      (set `self.isReady` true)
      (`KismetSystemLibrary.PrintString` "Platform is ready!")
      (`PrimitiveComponent.SetMaterial` (`self.Platform`) 0 "/Game/Materials/MI_PlatformReady.MI_PlatformReady"))))

(fn `UserConstructionScript`)