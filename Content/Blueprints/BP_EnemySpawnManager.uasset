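; Enemy wave manager that starts a new wave once no BP_Enemy actors remain in the level.
; NewEnemyWaveCheck, called with a transform, counts live enemies and, if none are left, triggers SpawnNewEnemies and drops a BP_Key at that transform.
; SpawnNewEnemies waits through a fixed delay, then tells every BP_EnemySpawner in the level to spawn an enemy.
; Debug prints report spawner count and wave progress.
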(event `self.ReceiveBeginPlay`
  (`KismetSystemLibrary.PrintString` "Spawn Manager is active")
  (bind _outactors (`GameplayStatics.GetAllActorsOfClass` "/Game/Blueprints/BP_EnemySpawner.BP_EnemySpawner_C"))
  (`KismetSystemLibrary.PrintString` (`KismetStringLibrary.Concat_StrStr` "There are " (`KismetStringLibrary.Conv_IntToString` (`KismetArrayLibrary.Array_Length` _outactors)) " spawners in the level." " There are " "##" " enemies in the level") true true (struct :`R` 1.0 :`G` 0.93319 :`A` 1.0) 10.0))

(event `NewEnemyWaveCheck`
  (params (Transform :type "Transform Structure"))
  (`KismetSystemLibrary.PrintString` "Checking enemy count")
  (bind _outactors (`GameplayStatics.GetAllActorsOfClass` "/Game/Blueprints/BP_Enemy.BP_Enemy_C"))
  (if (> (`KismetArrayLibrary.Array_Length` _outactors) 0)
    (`KismetSystemLibrary.PrintString` "There are still more enemies in the level")
    (else
      (`self.Spawn New Enemies`)
      (`|SpawnActorFromClass` "/Game/Blueprints/BP_Key.BP_Key_C" Transform "Undefined" "OverrideRootScale" null null))))

(event `Spawn New Enemies`
  (`KismetSystemLibrary.PrintString` "Spawning in new enemies in 10 seconds" true true (struct :`R` 1.0 :`B` 0.515838 :`A` 1.0))
  (`KismetSystemLibrary.Delay` 10.0)
  (bind _outactors (`GameplayStatics.GetAllActorsOfClass` "/Game/Blueprints/BP_EnemySpawner.BP_EnemySpawner_C"))
  (for (_array_element _array_index) _outactors
    (`/Game/Blueprints/BP_EnemySpawner.SpawnNewEnemy` _array_element)
    (`KismetSystemLibrary.PrintString` (`KismetStringLibrary.Concat_StrStr` (`KismetStringLibrary.Conv_IntToString` _array_index) "" (`KismetSystemLibrary.GetDisplayName` _array_element) "is spawning...")))
  (`KismetSystemLibrary.PrintString` "New wave complete!"))

(fn `UserConstructionScript`)